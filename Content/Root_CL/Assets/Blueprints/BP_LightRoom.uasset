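; BP_LightRoom is a red-light/green-light room that cycles a mesh material and spotlight color through green, yellow and red.
; Chained custom events with timed delays loop endlessly from BeginPlay, setting a Red flag during the red phase.
; Box overlap sets Inside five seconds after the player character enters and clears it on exit.
; Hit by the player character while Red and Inside only prints a debug string.
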(event OnComponentBeginOverlap(Box)
  (params (OverlappedComponent :type Primitive%20Component%20Object%20Reference) (OtherActor :type Actor%20Object%20Reference) (OtherComp :type Primitive%20Component%20Object%20Reference) (OtherBodyIndex :type Integer) (bFromSweep :type Boolean) (SweepResult :type Hit%20Result%20Structure%20%28by%20ref%29))
  (Utilities|Casting|CastToCore_PlayerCharacter OtherActor)
  (Utilities|FlowControl|Delay 5.0)
  (Variables|Default|SetbInside true))

(event OnComponentEndOverlap(Box)
  (params (OverlappedComponent :type Primitive%20Component%20Object%20Reference) (OtherActor :type Actor%20Object%20Reference) (OtherComp :type Primitive%20Component%20Object%20Reference) (OtherBodyIndex :type Integer))
  (Utilities|Casting|CastToCore_PlayerCharacter OtherActor)
  (Variables|Default|SetbInside false))

(event Custom|GreenLight
  (Rendering|Material|SetMaterial (Variables|Default|GetStaticMesh) 0 "/Game/Root_CL/Assets/Materials/M_Color_Green_Inst.M_Color_Green_Inst")
  (Rendering|Components|Light|SetLightColor (Variables|Default|GetSpotLight) "(R=0.000000,G=1.000000,B=0.052205,A=1.000000)" true)
  (Variables|Default|SetbRed false)
  (Utilities|FlowControl|Delay 2.0)
  (CallFunction|YellowLight))

(event Custom|YellowLight
  (Rendering|Material|SetMaterial (Variables|Default|GetStaticMesh) 0 "/Game/Root_CL/Assets/Materials/M_Color_Yellow_Inst.M_Color_Yellow_Inst")
  (Rendering|Components|Light|SetLightColor (Variables|Default|GetSpotLight) "(R=1.000000,G=0.904464,B=0.000000,A=1.000000)" true)
  (Utilities|FlowControl|Delay 1.0)
  (CallFunction|RedLight))

(event Custom|RedLight
  (Rendering|Material|SetMaterial (Variables|Default|GetStaticMesh) 0 "/Game/Root_CL/Assets/Materials/M_Color_Red_Inst.M_Color_Red_Inst")
  (Rendering|Components|Light|SetLightColor (Variables|Default|GetSpotLight) "(R=1.000000,G=0.023153,B=0.000000,A=1.000000)" true)
  (Variables|Default|SetbRed true)
  (Utilities|FlowControl|Delay 3.0)
  (CallFunction|GreenLight))

(event EventBeginPlay
  (CallFunction|GreenLight))

(event Collision|EventHit
  (params (MyComp :type Primitive%20Component%20Object%20Reference) (Other :type Actor%20Object%20Reference) (OtherComp :type Primitive%20Component%20Object%20Reference) (bSelfMoved :type Boolean) (HitLocation :type Vector :default "0, 0, 0") (HitNormal :type Vector :default "0, 0, 0") (NormalImpulse :type Vector :default "0, 0, 0") (Hit :type Hit%20Result%20Structure%20%28by%20ref%29))
  (Utilities|Casting|CastToCore_PlayerCharacter Other)
  (if (and (Variables|Default|GetbRed) (Variables|Default|GetbInside))
    (Development|PrintString "dod")))

(fn ConstructionScript)