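; BP_SplinePatrol is a patrolling detector that moves along a looping spline route and reacts to the player.
; Tick advances a distance along PatrolRoute at constant Speed, wrapping to zero at the end, and places ConePivot at that location and rotation.
; When Core_PlayerCharacter overlaps Trigger, the patrol pauses and the SpotLight turns red.
; When the overlap ends, the light turns green and the patrol resumes, with debug prints on both events.
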(event OnComponentBeginOverlap(Trigger)
  (params (OverlappedComponent :type Primitive%20Component%20Object%20Reference) (OtherActor :type Actor%20Object%20Reference) (OtherComp :type Primitive%20Component%20Object%20Reference) (OtherBodyIndex :type Integer) (bFromSweep :type Boolean) (SweepResult :type Hit%20Result%20Structure%20%28by%20ref%29))
  ;[1 1 1] Detecting player
  (Utilities|Casting|CastToCore_PlayerCharacter OtherActor)
  (Development|PrintString "DETECTED" true true "(R=1.000000,G=0.000000,B=0.008058,A=1.000000)")
  (Rendering|Components|Light|SetLightColor (Variables|Default|GetSpotLight) "(R=1.000000,G=0.001821,B=0.001821,A=1.000000)" true)
  (Variables|Default|SetbDetected true))

(event OnComponentEndOverlap(Trigger)
  (params (OverlappedComponent :type Primitive%20Component%20Object%20Reference) (OtherActor :type Actor%20Object%20Reference) (OtherComp :type Primitive%20Component%20Object%20Reference) (OtherBodyIndex :type Integer))
  ;[1 1 1] Detecting player
  (Utilities|Casting|CastToCore_PlayerCharacter OtherActor)
  (Development|PrintString "Gone")
  (Rendering|Components|Light|SetLightColor (Variables|Default|GetSpotLight) "(R=0.000000,G=1.000000,B=0.058824,A=1.000000)" true)
  (Variables|Default|SetbDetected false))

(event EventTick
  (params (DeltaSeconds :type Float%20%28single-precision%29))
  (bind _patrolroute (Variables|Default|GetPatrolRoute))
  (bind _patrolroute_2 (Variables|Default|GetPatrolRoute))
  (bind _returnvalue (Spline|GetSplineLength _patrolroute_2))
  ;[1 1 1] Rotating on spline
  (if (not (Variables|Default|GetbDetected))
    (if (>= (Variables|Default|GetCurrentDistanceOnSPline) _returnvalue)
      (Variables|Default|SetCurrentDistanceOnSPline 0.0)
      (else
        (Variables|Default|SetCurrentDistanceOnSPline (Math|Interpolation|FInterptoConstant (Variables|Default|GetCurrentDistanceOnSPline) _returnvalue (Utilities|Time|GetWorldDeltaSeconds) (Variables|Default|GetSpeed)))))
    (Transformation|SetRelativeLocationAndRotation (Variables|Default|GetConePivot) (Spline|GetLocationatDistanceAlongSpline _patrolroute (Variables|Default|GetCurrentDistanceOnSPline) "Local") (Spline|GetRotationatDistanceAlongSpline _patrolroute (Variables|Default|GetCurrentDistanceOnSPline) "Local") false false)))

(fn ConstructionScript)