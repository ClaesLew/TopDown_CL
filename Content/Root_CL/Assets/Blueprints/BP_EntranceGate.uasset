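; BP_EntranceGate is an entrance gate Blueprint that slides its Door component open and closed on demand.
; Open plays the OpenDoor timeline at PlayrateOpen, lerping the door's relative location from a fixed raised offset to EndPos.
; Close reverses the same timeline at PlayrateClose, so opening and closing can run at different speeds.
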(event Custom|Open
  (Components|Timeline|SetPlayRate (Variables|Default|GetOpenDoor) (Variables|Default|GetPlayrateOpen))
  (bind _alpha (Timeline|OpenDoor Play)
    (:Update
      (Transformation|SetRelativeLocation (Variables|Default|GetDoor) (Math|Vector|Lerp(Vector) "0, 0,150.000000" (Variables|Default|GetEndPos) _alpha) false false))))

(event Custom|Close
  (Components|Timeline|SetPlayRate (Variables|Default|GetOpenDoor) (Variables|Default|GetPlayrateClose))
  (bind _alpha (Timeline|OpenDoor Reverse)
    (:Update
      (Transformation|SetRelativeLocation (Variables|Default|GetDoor) (Math|Vector|Lerp(Vector) "0, 0,150.000000" (Variables|Default|GetEndPos) _alpha) false false))))

(fn ConstructionScript)