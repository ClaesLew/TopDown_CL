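; BP_MummyGuard is a guard whose detection cone kills the player on overlap and turns its spotlight red.
; Goats or other actors entering DetectZone add a point to PatrolRoute at runtime, setting Detected or Alert; investigated goats are destroyed after a delay.
; Tick moves ConePivot along that spline, closes the loop to return after a pause, then resets the route.
; The DetectZone lowering timeline is unconnected.
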(event OnComponentBeginOverlap(Trigger)
  (params (OverlappedComponent :type Primitive%20Component%20Object%20Reference) (OtherActor :type Actor%20Object%20Reference) (OtherComp :type Primitive%20Component%20Object%20Reference) (OtherBodyIndex :type Integer) (bFromSweep :type Boolean) (SweepResult :type Hit%20Result%20Structure%20%28by%20ref%29))
  ;[1 1 1] Detecting player
  (bind _ascore_player_character (Utilities|Casting|CastToCore_PlayerCharacter OtherActor))
  (Default|DEAD _ascore_player_character)
  (Development|PrintString "DETECTED" true true "(R=1.000000,G=0.000000,B=0.008058,A=1.000000)")
  (Rendering|Components|Light|SetLightColor (Variables|Default|GetSpotLight) "(R=1.000000,G=0.001821,B=0.001821,A=1.000000)" true))

(event OnComponentEndOverlap(Trigger)
  (params (OverlappedComponent :type Primitive%20Component%20Object%20Reference) (OtherActor :type Actor%20Object%20Reference) (OtherComp :type Primitive%20Component%20Object%20Reference) (OtherBodyIndex :type Integer))
  ;[1 1 1] Detecting player
  (Utilities|Casting|CastToCore_PlayerCharacter OtherActor)
  (Development|PrintString "Gone")
  (Rendering|Components|Light|SetLightColor (Variables|Default|GetSpotLight) "(R=0.000000,G=1.000000,B=0.058824,A=1.000000)" true))

(event OnComponentBeginOverlap(DetectZone)
  (params (OverlappedComponent :type Primitive%20Component%20Object%20Reference) (OtherActor :type Actor%20Object%20Reference) (OtherComp :type Primitive%20Component%20Object%20Reference) (OtherBodyIndex :type Integer) (bFromSweep :type Boolean) (SweepResult :type Hit%20Result%20Structure%20%28by%20ref%29))
  ;[1 1 1] I'm detecting something and need to scout
  (bind _asbp_goat (Utilities|Casting|CastToBP_Goat OtherActor)
    (:then
      (if (== (Spline|GetNumberOfSplinePoints (Variables|Default|GetPatrolRoute)) 1)
        (Utilities|FlowControl|Delay 0.3)
        (Variables|Default|SetActorPos (+ (Variables|/Script/Engine.SceneComponent|GetRelativeLocation (Variables|/Game/Root_CL/Assets/Blueprints/BP_Goat.BP_Goat_C|GetBody _asbp_goat)) "0, 0,150.000000"))
        (Variables|Default|SetbDetected true)
        (Spline|AddSplinePoint (Variables|Default|GetPatrolRoute) (stale _output_get_2) "World" true :!label _label)
        (if (Variables|Default|GetbDetected)
          (Utilities|FlowControl|Delay 4.0)
          (Actor|DestroyActor _asbp_goat))))
    (:CastFailed
      (bind _output_get (Variables|Default|SetActorRef OtherActor))
      (if (not (Variables|Default|GetbDetected))
        (Development|PrintString "Hello")
        (Development|PrintString (Utilities|String|ToString(Vector) (Transformation|GetActorLocation _output_get)))
        (bind _output_get_2 (Variables|Default|SetActorPos (+ (Transformation|GetActorLocation _output_get) "0, 0,150.000000")))
        (Variables|Default|SetbAlert true)
        (goto _label)))))

(event EventTick
  (params (DeltaSeconds :type Float%20%28single-precision%29))
  (bind _patrolroute (Variables|Default|GetPatrolRoute))
  (bind _patrolroute_2 (Variables|Default|GetPatrolRoute))
  (bind _patrolroute_3 (Variables|Default|GetPatrolRoute))
  (bind _returnvalue (Spline|GetSplineLength _patrolroute_2))
  ;[1 1 1] Rotating on spline
  (if (Variables|Default|GetbDetected)
    (if (>= (Variables|Default|GetCurrentDistanceOnSPline) _returnvalue) :!label _label
      (Utilities|FlowControl|Delay 4.0)
      (Spline|SetClosedLoop (Variables|Default|GetPatrolRoute) true true)
      (Development|PrintString "funka")
      (if (>= (Variables|Default|GetCurrentDistanceOnSPline) _returnvalue)
        (Variables|Default|SetCurrentDistanceOnSPline 0.0)
        (Spline|ClearSplinePoints _patrolroute_3 true)
        (Spline|AddSplinePoint _patrolroute_3 (Math|Vector|MakeVector 0.0 0.0 0.0) "Local" true)
        (Spline|SetClosedLoop _patrolroute_3 false true)
        (Variables|Default|SetbDetected false)
        (Variables|Default|SetbAlert false)
        (else
          (Variables|Default|SetCurrentDistanceOnSPline (Math|Interpolation|FInterptoConstant (Variables|Default|GetCurrentDistanceOnSPline) _returnvalue (Utilities|Time|GetWorldDeltaSeconds) (Variables|Default|GetSpeed)) :!label _label_2)))
      (else
        (goto _label_2)))
    (Transformation|SetRelativeLocationAndRotation (Variables|Default|GetConePivot) (Spline|GetLocationatDistanceAlongSpline _patrolroute (Variables|Default|GetCurrentDistanceOnSPline) "Local") (Spline|GetRotationatDistanceAlongSpline _patrolroute (Variables|Default|GetCurrentDistanceOnSPline) "Local") false false)
    (elif (Variables|Default|GetbAlert)
      (goto _label))))

(event EventBeginPlay
  (Variables|Default|SetDetectStartPos (Transformation|GetWorldLocation (Variables|Default|GetDetectZone))))

(fn ConstructionScript)