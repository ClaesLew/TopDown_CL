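; BP_PreassurePLate is a pressure plate that opens its linked BP_EntranceGate while held down and closes it on release.
; With no ActorRef set, the player's overlap activates it; otherwise only that referenced BP_Keystone does, provided its Keystone1 or Keystone2 flag is set.
; Trigger begin and end overlaps play and reverse a timeline that lerps the Button's height, then call the gate's Open or Close.
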(event OnComponentBeginOverlap(Trigger)
  (params (OverlappedComponent :type Primitive%20Component%20Object%20Reference) (OtherActor :type Actor%20Object%20Reference) (OtherComp :type Primitive%20Component%20Object%20Reference) (OtherBodyIndex :type Integer) (bFromSweep :type Boolean) (SweepResult :type Hit%20Result%20Structure%20%28by%20ref%29))
  (Utilities|Casting|CastToCore_PlayerCharacter OtherActor
    (:then
      (if (== (Variables|Default|GetActorRef) 0)
        (CallFunction|PushDown :!label _label)
        (bind _asbp_entrance_gate (Utilities|Casting|CastToBP_EntranceGate (Variables|Default|GetDoorRef)))
        (Default|Open _asbp_entrance_gate)
        (else
          (bind _asbp_keystone (Utilities|Casting|CastToBP_Keystone OtherActor :!label _label_2))
          (if (== _asbp_keystone (Variables|Default|GetActorRef))
            (if (Variables|/Game/Root_CL/Assets/Blueprints/BP_Keystone.BP_Keystone_C|GetbKeystone1 _asbp_keystone)
              (goto _label)
              (elif (Variables|/Game/Root_CL/Assets/Blueprints/BP_Keystone.BP_Keystone_C|GetbKeystone2 _asbp_keystone)
                (goto _label)))))))
    (:CastFailed
      (goto _label_2))))

(event OnComponentEndOverlap(Trigger)
  (params (OverlappedComponent :type Primitive%20Component%20Object%20Reference) (OtherActor :type Actor%20Object%20Reference) (OtherComp :type Primitive%20Component%20Object%20Reference) (OtherBodyIndex :type Integer))
  (Utilities|Casting|CastToCore_PlayerCharacter OtherActor
    (:then
      (if (== (Variables|Default|GetActorRef) 0)
        (CallFunction|PushUp :!label _label)
        (bind _asbp_entrance_gate (Utilities|Casting|CastToBP_EntranceGate (Variables|Default|GetDoorRef)))
        (Default|Close _asbp_entrance_gate)
        (else
          (bind _asbp_keystone (Utilities|Casting|CastToBP_Keystone OtherActor :!label _label_2))
          (if (== _asbp_keystone (Variables|Default|GetActorRef))
            (if (Variables|/Game/Root_CL/Assets/Blueprints/BP_Keystone.BP_Keystone_C|GetbKeystone1 _asbp_keystone)
              (goto _label)
              (elif (Variables|/Game/Root_CL/Assets/Blueprints/BP_Keystone.BP_Keystone_C|GetbKeystone2 _asbp_keystone)
                (goto _label)))))))
    (:CastFailed
      (goto _label_2))))

(event Custom|PushDown
  (bind _newtrack_0 (Timeline|Pushing%20down Play)
    (:Update
      (Transformation|SetRelativeLocation (Variables|Default|GetButton) (Math|Vector|Lerp(Vector) "0, 0,15.000000" "0, 0,-10.000000" _newtrack_0) false false))))

(event Custom|PushUp
  (bind _newtrack_0 (Timeline|Pushing%20down Reverse)
    (:Update
      (Transformation|SetRelativeLocation (Variables|Default|GetButton) (Math|Vector|Lerp(Vector) "0, 0,15.000000" "0, 0,-10.000000" _newtrack_0) false false))))

(event EventBeginPlay)

(fn ConstructionScript)