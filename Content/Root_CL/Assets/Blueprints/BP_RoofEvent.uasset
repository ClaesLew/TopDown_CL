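; BP_RoofEvent is a three-round boulder hazard, apparently falling from the roof, that destroys itself after the last round.
; Once START is set, Tick kicks off the rounds and keeps a different subset of meshes hidden and non-colliding each round.
; BeginRound moves Boulder2 with a two-track timeline, then re-enables the meshes and recurses for the next round.
; Player overlaps with the meshes only print a debug hit message.
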(event OnComponentBeginOverlap(StaticMesh5)
  (params (OverlappedComponent :type Primitive%20Component%20Object%20Reference) (OtherActor :type Actor%20Object%20Reference) (OtherComp :type Primitive%20Component%20Object%20Reference) (OtherBodyIndex :type Integer) (bFromSweep :type Boolean) (SweepResult :type Hit%20Result%20Structure%20%28by%20ref%29))
  ;[1 1 1] Boulder hits player
  (Utilities|Casting|CastToCore_PlayerCharacter OtherActor)
  (Development|PrintString "TRAFFAD"))

(event OnComponentBeginOverlap(Boulder2)
  (params (OverlappedComponent :type Primitive%20Component%20Object%20Reference) (OtherActor :type Actor%20Object%20Reference) (OtherComp :type Primitive%20Component%20Object%20Reference) (OtherBodyIndex :type Integer) (bFromSweep :type Boolean) (SweepResult :type Hit%20Result%20Structure%20%28by%20ref%29))
  ;[1 1 1] Boulder hits player
  (Utilities|Casting|CastToCore_PlayerCharacter OtherActor)
  (Development|PrintString "TRAFFAD"))

(event OnComponentBeginOverlap(StaticMesh10)
  (params (OverlappedComponent :type Primitive%20Component%20Object%20Reference) (OtherActor :type Actor%20Object%20Reference) (OtherComp :type Primitive%20Component%20Object%20Reference) (OtherBodyIndex :type Integer) (bFromSweep :type Boolean) (SweepResult :type Hit%20Result%20Structure%20%28by%20ref%29))
  ;[1 1 1] Boulder hits player
  (Utilities|Casting|CastToCore_PlayerCharacter OtherActor)
  (Development|PrintString "TRAFFAD"))

(event OnComponentBeginOverlap(StaticMesh1)
  (params (OverlappedComponent :type Primitive%20Component%20Object%20Reference) (OtherActor :type Actor%20Object%20Reference) (OtherComp :type Primitive%20Component%20Object%20Reference) (OtherBodyIndex :type Integer) (bFromSweep :type Boolean) (SweepResult :type Hit%20Result%20Structure%20%28by%20ref%29))
  ;[1 1 1] Boulder hits player
  (Utilities|Casting|CastToCore_PlayerCharacter OtherActor)
  (Development|PrintString "TRAFFAD"))

(event OnComponentBeginOverlap(StaticMesh3)
  (params (OverlappedComponent :type Primitive%20Component%20Object%20Reference) (OtherActor :type Actor%20Object%20Reference) (OtherComp :type Primitive%20Component%20Object%20Reference) (OtherBodyIndex :type Integer) (bFromSweep :type Boolean) (SweepResult :type Hit%20Result%20Structure%20%28by%20ref%29))
  ;[1 1 1] Boulder hits player
  (Utilities|Casting|CastToCore_PlayerCharacter OtherActor)
  (Development|PrintString "TRAFFAD"))

(event OnComponentBeginOverlap(StaticMesh4)
  (params (OverlappedComponent :type Primitive%20Component%20Object%20Reference) (OtherActor :type Actor%20Object%20Reference) (OtherComp :type Primitive%20Component%20Object%20Reference) (OtherBodyIndex :type Integer) (bFromSweep :type Boolean) (SweepResult :type Hit%20Result%20Structure%20%28by%20ref%29))
  ;[1 1 1] Boulder hits player
  (Utilities|Casting|CastToCore_PlayerCharacter OtherActor)
  (Development|PrintString "TRAFFAD"))

(event OnComponentBeginOverlap(StaticMesh11)
  (params (OverlappedComponent :type Primitive%20Component%20Object%20Reference) (OtherActor :type Actor%20Object%20Reference) (OtherComp :type Primitive%20Component%20Object%20Reference) (OtherBodyIndex :type Integer) (bFromSweep :type Boolean) (SweepResult :type Hit%20Result%20Structure%20%28by%20ref%29))
  ;[1 1 1] Boulder hits player
  (Utilities|Casting|CastToCore_PlayerCharacter OtherActor)
  (Development|PrintString "TRAFFAD"))

(event OnComponentBeginOverlap(StaticMesh6)
  (params (OverlappedComponent :type Primitive%20Component%20Object%20Reference) (OtherActor :type Actor%20Object%20Reference) (OtherComp :type Primitive%20Component%20Object%20Reference) (OtherBodyIndex :type Integer) (bFromSweep :type Boolean) (SweepResult :type Hit%20Result%20Structure%20%28by%20ref%29))
  ;[1 1 1] Boulder hits player
  (Utilities|Casting|CastToCore_PlayerCharacter OtherActor)
  (Development|PrintString "TRAFFAD"))

(event OnComponentBeginOverlap(StaticMesh7)
  (params (OverlappedComponent :type Primitive%20Component%20Object%20Reference) (OtherActor :type Actor%20Object%20Reference) (OtherComp :type Primitive%20Component%20Object%20Reference) (OtherBodyIndex :type Integer) (bFromSweep :type Boolean) (SweepResult :type Hit%20Result%20Structure%20%28by%20ref%29))
  ;[1 1 1] Boulder hits player
  (Utilities|Casting|CastToCore_PlayerCharacter OtherActor)
  (Development|PrintString "TRAFFAD"))

(event OnComponentBeginOverlap(StaticMesh8)
  (params (OverlappedComponent :type Primitive%20Component%20Object%20Reference) (OtherActor :type Actor%20Object%20Reference) (OtherComp :type Primitive%20Component%20Object%20Reference) (OtherBodyIndex :type Integer) (bFromSweep :type Boolean) (SweepResult :type Hit%20Result%20Structure%20%28by%20ref%29))
  ;[1 1 1] Boulder hits player
  (Utilities|Casting|CastToCore_PlayerCharacter OtherActor)
  (Development|PrintString "TRAFFAD"))

(event OnComponentBeginOverlap(StaticMesh9)
  (params (OverlappedComponent :type Primitive%20Component%20Object%20Reference) (OtherActor :type Actor%20Object%20Reference) (OtherComp :type Primitive%20Component%20Object%20Reference) (OtherBodyIndex :type Integer) (bFromSweep :type Boolean) (SweepResult :type Hit%20Result%20Structure%20%28by%20ref%29))
  ;[1 1 1] Boulder hits player
  (Utilities|Casting|CastToCore_PlayerCharacter OtherActor)
  (Development|PrintString "TRAFFAD"))

(event Custom|BeginRound
  (bind _boulder2 (Variables|Default|GetBoulder2))
  (bind _boulder2_2 (Variables|Default|GetBoulder2))
  (bind _rounds (Variables|Default|GetRounds))
  (bind _staticmesh1 (Variables|Default|GetStaticMesh1))
  (bind _relativelocation (Variables|/Script/Engine.SceneComponent|GetRelativeLocation _boulder2_2))
  ;[1 1 1] Round Starts
  (Utilities|FlowControl|Delay 2.0)
  (bind (_direction _track1 _track2) (Timeline|Timeline_0 PlayFromStart)
    (:Update
      (Transformation|SetRelativeLocation _boulder2 (Math|Vector|Lerp(Vector) _relativelocation "-150.000000,-300.000000, 0" _track1) false false)
      (Transformation|SetRelativeLocation _boulder2 (Math|Vector|Lerp(Vector) _relativelocation "-150.000000,-300.000000,500.000000" _track2) false false))
    (:Finished
      (Development|PrintString "KLar")
      (Utilities|FlowControl|Delay 2.0)
      (Math|Integer|IncrementInt _rounds
        (:%20%20
          (if (<= _rounds 3)
            (Collision|SetCollisionEnabled _staticmesh1 "QueryOnly")
            (Rendering|SetVisibility _staticmesh1 true false)
            (CallFunction|BeginRound)
            (else
              (Actor|DestroyActor))))))))

(event EventTick
  (params (DeltaSeconds :type Float%20%28single-precision%29))
  (bind _staticmesh5 (Variables|Default|GetStaticMesh5))
  (bind _staticmesh11 (Variables|Default|GetStaticMesh11))
  (bind _staticmesh1 (Variables|Default|GetStaticMesh1))
  ;[1 1 1] What Round is it?
  (if (Variables|Default|GetbSTART)
    (switch int (Variables|Default|GetRounds)
      (:0
        (Utilities|FlowControl|Delay 2.0)
        (Math|Integer|IncrementInt (Variables|Default|GetRounds)
          (:%20%20
            (CallFunction|BeginRound))))
      (:1
        (Rendering|SetVisibility _staticmesh5 false false)
        (Collision|SetCollisionEnabled _staticmesh5 "NoCollision"))
      (:2
        (Rendering|SetVisibility _staticmesh11 false false)
        (Collision|SetCollisionEnabled _staticmesh11 "NoCollision"))
      (:3
        (Rendering|SetVisibility _staticmesh1 false false)
        (Collision|SetCollisionEnabled _staticmesh1 "NoCollision")))))

(fn ConstructionScript)